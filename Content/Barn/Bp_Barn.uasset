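; Barn actor that stores a quantity for each plant type in the Stokage map, keyed by the Plantes enum.
; BeginPlay seeds every enum entry at zero, then calls ShowDictionary to print each type and count on screen.
; The AddElement event increases a plant's stored count by a given quantity.
; A delayed test that adds one plant and reprints the map is left disconnected.
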(event `self.ReceiveBeginPlay`
  (bind _enumvalue (foreach `/Game/Barn/Plantes` true)
    (:`LoopBody`
      (`BlueprintMapLibrary.Map_Add` (`self.Stokage`) _enumvalue))
    (:`then`
      (`self.ShowDictionary`))))

(event `self.ReceiveTick`
  (params (DeltaSeconds :type "Float (single-precision)")))

(event `AddElement`
  (params (Plante :type "/Game/Barn/Plantes Enum" :default "NewEnumerator0") (Quantite :type Integer))
  (bind _stokage (`self.Stokage`))
  (`BlueprintMapLibrary.Map_Add` _stokage Plante (+ Quantite (`BlueprintMapLibrary.Map_Find` _stokage Plante))))

(fn `ShowDictionary`
  (bind _stokage (`self.Stokage`))
  (bind _keys (`BlueprintMapLibrary.Map_Keys` _stokage))
  (for _array_element _keys
    (`KismetSystemLibrary.PrintString` (`KismetStringLibrary.BuildString_Int` (`|GetEnumeratorNameAsString` _array_element) " : " (`BlueprintMapLibrary.Map_Find` _stokage _array_element)) true true (struct :`G` 0.66 :`B` 1.0 :`A` 1.0) 1.0)))

(fn `UserConstructionScript`)