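; Plant actor that grows through three visual stages while it has water.
; Tick drains irrigation and advances a growth timer, both scaled by a fertilizer multiplier that resets to normal when its countdown expires.
; Each completed timer shows the next stage component and hides the others.
; AddIrrigation adds water up to a maximum and refreshes the irrigation widget's bar, which is not updated as water drains.
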(event `self.ReceiveBeginPlay`
  (`KismetArrayLibrary.Array_Add` (`self.PlantStat`) (`self.LV1`))
  (`KismetArrayLibrary.Array_Add` (`self.PlantStat`) (`self.LV2`))
  (`KismetArrayLibrary.Array_Add` (`self.PlantStat`) (`self.LV3`))
  (`self.ChangeState` 0)
  (if (== (`self.GrowTime`) 0.0)
    (set `self.GrowTime` 2.0))
  (bind _aswdg_irrigation (cast `/Game/Plantes/blueprints/Widget/WDG_Irrigation` (`WidgetComponent.GetUserWidgetObject` (`self.Widget`))))
  (set `self.WDG_Irrigation` _aswdg_irrigation)
  (`self.SetWaterBar`))

(event `self.ReceiveTick`
  (params (DeltaSeconds :type "Float (single-precision)"))
  (bind _irrigation (`self.Irrigation`))
  (bind _returnvalue (* DeltaSeconds (`self.FertilizerMultiplier `)))
  (if (>= _irrigation 0.0)
    (set `self.Irrigation` (- _irrigation _returnvalue))
    (`self.FertilizeCountDown` DeltaSeconds
      (:`Out`
        (bind _output_get (set `self.ActualGrow` (+ _returnvalue (`self.ActualGrow`))))
        (if (>= _output_get (`self.GrowTime`))
          (set `self.ActualGrow` 0.0)
          (if (< (`self.State`) (- (`KismetArrayLibrary.Array_Length` (`self.PlantStat`)) 1))
            (bind _result (`/Engine/EditorBlueprintResources/StandardMacros.IncrementInt` (`self.State`))
              (:`  `
                (`self.ChangeState` _result)))))))))

(event `AddIrrigation`
  (params (Value :type "Float (double-precision)"))
  (bind _output_get (set `self.Irrigation` (+ Value (`self.Irrigation`))))
  (if (> _output_get (`self.MaxIrrigation`))
    (set `self.Irrigation` (`self.MaxIrrigation`)))
  (`self.SetWaterBar`))

(fn `ChangeState`
  (params (State :type Integer))
  (for (_array_element _array_index) (`self.PlantStat`)
    (`SceneComponent.SetVisibility` _array_element (== _array_index State) true)))

(fn `UserConstructionScript`)